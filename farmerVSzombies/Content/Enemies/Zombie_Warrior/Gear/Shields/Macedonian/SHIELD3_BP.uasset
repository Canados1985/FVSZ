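; Macedonian shield gear for the zombie warrior enemy that absorbs bullets until it breaks.
; Overlapping an actor tagged BULLET plays a metal impact sound, lowers Durability and briefly flashes both mesh parts to transparent materials.
; Tick polls Durability and, once it reaches zero or below, a DoOnce plays a destruction sound and destroys the actor after a short delay.
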(event EventBeginPlay)

(event Collision|EventActorBeginOverlap
  (params (OtherActor :type Actor%20Object%20Reference))
  (if (Actor|ActorHasTag OtherActor "BULLET")
    (Audio|PlaySoundatLocation "/Game/Enemies/Zombie_Warrior/Sound/metal_shied_vs_bullet2_Cue.metal_shied_vs_bullet2_Cue" (Transformation|GetWorldLocation (Variables|Default|Getarmsofsparta_3071)) "0, 0, 0" 2.0)
    (Rendering|Material|SetMaterial (Variables|Default|Getarmsofsparta_4535) 0 "/Game/Enemies/Zombie_Warrior/Gear/Shields/Macedonian/4535Mat_Transparent.4535Mat_Transparent")
    (Rendering|Material|SetMaterial (Variables|Default|Getarmsofsparta_3071) 0 "/Game/Enemies/Zombie_Warrior/Gear/Shields/Macedonian/3071Mat_Transparent.3071Mat_Transparent")
    (Variables|Default|SetDurability (- (Variables|Default|GetDurability) 25))
    (Utilities|FlowControl|Delay 0.2)
    (Rendering|Material|SetMaterial (Variables|Default|Getarmsofsparta_4535) 0 "/Game/Enemies/Zombie_Warrior/Gear/Shields/Macedonian/4535Mat.4535Mat")
    (Rendering|Material|SetMaterial (Variables|Default|Getarmsofsparta_3071) 0 "/Game/Enemies/Zombie_Warrior/Gear/Shields/Macedonian/3071Mat.3071Mat")))

(event EventTick
  (params (DeltaSeconds :type Float%20%28single-precision%29))
  (Math|Integer|CompareInt (Variables|Default|GetDurability)
    (:==
      _)
    (:<
      _))
  (Utilities|FlowControl|DoOnce false
    (:Completed
      (Audio|PlaySoundatLocation "/Game/Enemies/Zombie_Warrior/Sound/metalshield_destroyed_Cue.metalshield_destroyed_Cue" (Transformation|GetWorldLocation (Variables|Default|Getarmsofsparta_4535)) "0, 0, 0" 1e+01)
      (Utilities|FlowControl|Delay 0.3)
      (Actor|DestroyActor))))

(fn ConstructionScript)