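; SHIELD2_BP is a destructible shield actor in the Zombie Warrior enemy gear that loses durability when hit by bullets.
; An overlap with a BULLET-tagged actor plays an impact sound, subtracts durability and briefly swaps the shield mesh to a transparent material as a hit flash.
; Tick polls durability and, at zero or below, a DoOnce plays a destruction sound and destroys the actor after a short delay.
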(event EventBeginPlay)

(event Collision|EventActorBeginOverlap
  (params (OtherActor :type Actor%20Object%20Reference))
  (if (Actor|ActorHasTag OtherActor "BULLET")
    (Audio|PlaySoundatLocation "/Game/Enemies/Zombie_Warrior/Sound/metal_shied_vs_bullet2_Cue.metal_shied_vs_bullet2_Cue" (Transformation|GetWorldLocation (Variables|Default|GetWonder_Woman_V_Shield)) "0, 0, 0" 2.0)
    (Rendering|Material|SetMaterial (Variables|Default|GetWonder_Woman_V_Shield) 0 "/Game/Enemies/Zombie_Warrior/Gear/Shields/WWVshield_Transparent.WWVshield_Transparent")
    (Variables|Default|SetDurability (- (Variables|Default|GetDurability) 25))
    (Utilities|FlowControl|Delay 0.2)
    (Rendering|Material|SetMaterial (Variables|Default|GetWonder_Woman_V_Shield) 0 "/Game/Enemies/Zombie_Warrior/Gear/Shields/WWVshield.WWVshield")))

(event EventTick
  (params (DeltaSeconds :type Float%20%28single-precision%29))
  (Math|Integer|CompareInt (Variables|Default|GetDurability)
    (:==
      _)
    (:<
      _))
  (Utilities|FlowControl|DoOnce false
    (:Completed
      (Audio|PlaySoundatLocation "/Game/Enemies/Zombie_Warrior/Sound/metalshield_destroyed_Cue.metalshield_destroyed_Cue" (Transformation|GetWorldLocation (Variables|Default|GetWonder_Woman_V_Shield)) "0, 0, 0" 1e+01)
      (Utilities|FlowControl|Delay 0.3)
      (Actor|DestroyActor))))

(fn ConstructionScript)