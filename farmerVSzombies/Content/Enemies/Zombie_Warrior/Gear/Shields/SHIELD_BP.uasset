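; Zombie warrior wooden shield actor that absorbs bullet hits until it breaks.
; Overlaps with BULLET-tagged actors play an impact sound, reduce Durability and briefly swap the mesh to a transparent wood material as hit feedback.
; Tick polls Durability and, once it reaches zero or below, a DoOnce plays the destruction sound, sets WoodShieldIsDestroyed and destroys the actor after a tiny delay.
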(event EventBeginPlay)

(event Collision|EventActorBeginOverlap
  (params (OtherActor :type Actor%20Object%20Reference))
  (if (Actor|ActorHasTag OtherActor "BULLET")
    (Audio|PlaySoundatLocation "/Game/Enemies/Zombie_Warrior/Sound/wood_shied_vs_bullet_Cue.wood_shied_vs_bullet_Cue" (Transformation|GetWorldLocation (Variables|Default|Getshield_skandinav_medieval_02)) "0, 0, 0" 2.0)
    (Rendering|Material|SetMaterial (Variables|Default|Getshield_skandinav_medieval_02) 0 "/Game/Enemies/Zombie_Warrior/Gear/Shields/wood_Transparent.wood_Transparent")
    (Variables|Default|SetDurability (- (Variables|Default|GetDurability) 25))
    (Utilities|FlowControl|Delay 0.2)
    (Rendering|Material|SetMaterial (Variables|Default|Getshield_skandinav_medieval_02) 0 "/Game/Enemies/Zombie_Warrior/Gear/Shields/wood.wood")))

(event EventTick
  (params (DeltaSeconds :type Float%20%28single-precision%29))
  (Math|Integer|CompareInt (Variables|Default|GetDurability)
    (:==
      _)
    (:<
      _))
  (Utilities|FlowControl|DoOnce false
    (:Completed
      (Audio|PlaySoundatLocation "/Game/Enemies/Zombie_Warrior/Sound/shield_destroyed_Cue.shield_destroyed_Cue" (Transformation|GetWorldLocation (Variables|Default|Getshield_skandinav_medieval_02)) "0, 0, 0" 5.0)
      (Variables|Default|SetWoodShield_Is_Destroyed true)
      (Utilities|FlowControl|Delay 0.01)
      (Actor|DestroyActor))))

(fn ConstructionScript)