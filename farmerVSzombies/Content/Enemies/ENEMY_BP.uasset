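; Enemy Blueprint, apparently a parent class, that moves toward vegetables, fences and the player character on sight.
; PawnSensing's OnSeePawn feeds a Sequence that tries casts to VEGETABLES_BP, BP_FENCE and ThirdPersonCharacter.
; Each successful cast starts an AIMoveTo targeting that actor, with debug prints on the fence and player branches.
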(event OnSeePawn(PawnSensing)
  (params (Pawn :type Pawn%20Object%20Reference))
  (Utilities|FlowControl|Sequence
    (:then_0
      (bind _asvegetables_bp (Utilities|Casting|CastToVEGETABLES_BP Pawn))
      (AI|AIMoveTo self (Transformation|GetActorLocation _asvegetables_bp) _asvegetables_bp 5.0 false))
    (:then_1
      (bind _asbp_fence (Utilities|Casting|CastToBP_FENCE Pawn))
      (AI|AIMoveTo self (Transformation|GetActorLocation _asbp_fence) _asbp_fence 5.0 false
        (:then
          (Development|PrintString "FENCE IS WORKING PARENT CLASS"))))
    (:then_2
      (bind _asthird_person_character (Utilities|Casting|CastToThirdPersonCharacter Pawn))
      (AI|AIMoveTo self (Transformation|GetActorLocation _asthird_person_character) _asthird_person_character 1.0 false
        (:then
          (Development|PrintString "THEY SEE PLAYER"))))))

(event EventTick
  (params (DeltaSeconds :type Float%20%28single-precision%29)))

(fn ConstructionScript)